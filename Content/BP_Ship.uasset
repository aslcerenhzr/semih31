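; Ship actor that travels point to point along a randomly chosen BP_Spline and gets pulled toward a light's center when hit.
; On BeginPlay it finds the nearest spline point, eases onto it, then timelines lerp location through successive points, pausing between each.
; LightHit lerps it to the given center and sets IsFollowingLight, which the active spline movement never checks.
; An older loop-based movement that checks that flag is left disconnected.
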(event Custom|MoveSpline
  (bind _splineref (Variables|Default|GetSplineREF))
  (bind _lerp (Timeline|GoToNextSplineKey PlayFromStart)
    (:Update
      (Transformation|SetActorLocationAndRotation (Math|Vector|Lerp(Vector) (Utilities|Array|Get(acopy) (Variables|/Game/BP_Spline.BP_Spline_C|GetPointsLocation (Variables|Default|GetSplineREF)) (Variables|Default|GetPointIndex)) (Utilities|Array|Get(acopy) (Variables|/Game/BP_Spline.BP_Spline_C|GetPointsLocation _splineref) (+ (Variables|Default|GetPointIndex) 1)) _lerp) (Spline|GetRotationatSplinePoint (Variables|/Game/BP_Spline.BP_Spline_C|GetSpline _splineref) (+ (Variables|Default|GetPointIndex) 1) "Local")))
    (:Finished
      (bind _result (Math|Integer|IncrementInt (Variables|Default|GetPointIndex))
        (:%20%20
          (if (not (== (+ _result 1) (Spline|GetNumberOfSplinePoints (Variables|/Game/BP_Spline.BP_Spline_C|GetSpline (Variables|Default|GetSplineREF)))))
            (Utilities|FlowControl|Delay 2.0)
            (Timeline|GoToNextSplineKey PlayFromStart)))))))

(event Custom|MoveToSpline
  (bind _returnvalue (Transformation|GetActorLocation))
  (for (_array_element _array_index) (Variables|/Game/BP_Spline.BP_Spline_C|GetPointsLocation (Variables|Default|GetSplineREF))
    (if (< (Math|Vector|Distance(Vector) _array_element _returnvalue) (Variables|Default|GetDistToSpline))
      (Variables|Default|SetDistToSpline (Math|Vector|Distance(Vector) _array_element _returnvalue))
      (Variables|Default|SetClosesestPoint _array_element)
      (Variables|Default|SetPointIndex _array_index)))
  (Utilities|FlowControl|Delay 0.2)
  (bind _newtrack_0 (Timeline|Timeline_0 Play)
    (:Update
      (Transformation|SetActorLocation (Math|Vector|Lerp(Vector) _returnvalue (Variables|Default|GetClosesestPoint) _newtrack_0) false false))
    (:Finished
      (CallFunction|MoveSpline))))

(event EventLightNoHit
  (Variables|Default|SetisFollowingLight false))

(event EventBeginPlay
  (bind _returnvalue (Actor|GetActorOfClass "/Game/Light/BP_Light.BP_Light_C"))
  (Variables|Default|SetBP_Light _returnvalue)
  (bind _outactors (Actor|GetAllActorsOfClass "/Game/BP_Spline.BP_Spline_C"))
  (Variables|Default|SetSplineREF (.OutItem (Utilities|Array|Random _outactors)))
  (CallFunction|MovetoSpline))

(event EventLightHit
  (params (Center :type Vector :default "0, 0, 0"))
  (Variables|Default|SetisFollowingLight true)
  (Variables|Default|SetCurrentLoc (Transformation|GetActorLocation))
  (bind _gotocenter (Timeline|MoveToCenter PlayFromStart)
    (:Update
      (Transformation|SetActorLocation (Math|Vector|Lerp(Vector) (Variables|Default|GetCurrentLoc) Center _gotocenter) false false))))

(fn ConstructionScript)