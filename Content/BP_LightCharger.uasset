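; BP_LightCharger is an interactable actor that takes over the first-person player's view when used.
; It finds and caches the BP_FirstPersonCharacter on BeginPlay.
; On interact, it blends the player camera to itself, disables character movement by setting the movement mode to None, and switches the character's state enum.
; No charging logic or return to normal control is implemented here.
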(event Collision|EventActorBeginOverlap
  (params (OtherActor :type Actor%20Object%20Reference)))

(event EventTick
  (params (DeltaSeconds :type Float%20%28single-precision%29)))

(event EventOnInteract
  (Game|Player|SetViewTargetwithBlend (Game|GetPlayerController 0) self 1.2 "VTBlend_Linear" 0.0 true)
  (Pawn|Components|CharacterMovement|SetMovementMode (Variables|/Script/Engine.Character|GetCharacterMovement (Variables|Default|GetBP_FirstPersonCharacter)) "MOVE_None" 0)
  (Variables|/Game/FirstPerson/Blueprints/BP_FirstPersonCharacter.BP_FirstPersonCharacter_C|SetCurrentState (Variables|Default|GetBP_FirstPersonCharacter) "NewEnumerator1"))

(event EventBeginPlay
  (bind _returnvalue (Actor|GetActorOfClass "/Game/FirstPerson/Blueprints/BP_FirstPersonCharacter.BP_FirstPersonCharacter_C"))
  (Variables|Default|SetBP_FirstPersonCharacter _returnvalue))

(fn ConstructionScript)