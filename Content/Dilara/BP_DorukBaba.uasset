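; BP_DorukBaba is an interactable actor that sets itself active and blends the player's camera view to itself on interact.
; RotateXAxis and RotateYAxis both add their input to the Sphere's world pitch, clamped to ±90 before the addition, and zero roll and yaw.
; Box1 prints a debug message when it overlaps the Cone component.
; Tick checks the active flag but does nothing yet, and neither rotate function is called within this Blueprint.
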(event OnComponentBeginOverlap(Box1)
  (params (OverlappedComponent :type Primitive%20Component%20Object%20Reference) (OtherActor :type Actor%20Object%20Reference) (OtherComp :type Primitive%20Component%20Object%20Reference) (OtherBodyIndex :type Integer) (bFromSweep :type Boolean) (SweepResult :type Hit%20Result%20Structure%20%28by%20ref%29))
  (if (== OtherComp (Variables|Default|GetCone))
    (Development|PrintString "Hello")))

(event EventBeginPlay)

(event Collision|EventActorBeginOverlap
  (params (OtherActor :type Actor%20Object%20Reference)))

(event EventOnInteract
  (Variables|Default|SetisActive true)
  (Game|Player|SetViewTargetwithBlend (Game|GetPlayerController 0) self 1.5 "VTBlend_Linear" 0.0 false))

(event EventTick
  (params (DeltaSeconds :type Float%20%28single-precision%29))
  (if (Variables|Default|GetisActive)
    _))

(fn ConstructionScript)

(fn RotateYAxis
  (params (YAmount :type Float%20%28double-precision%29))
  (Variables|Default|SetRotationAmount YAmount)
  (Transformation|SetWorldRotation (Variables|Default|GetSphere) (Math|Rotator|MakeRotator 0.0 (+ (Variables|Default|GetRotationAmount) (Math|Float|Clamp(Float) (.pitch (Transformation|GetWorldRotation (Variables|Default|GetSphere))) -9e+01 9e+01)) 0.0) false false))

(fn RotateXAxis
  (params (XAmount :type Float%20%28double-precision%29))
  (Variables|Default|SetRotationAmount XAmount)
  (Transformation|SetWorldRotation (Variables|Default|GetSphere) (Math|Rotator|MakeRotator 0.0 (+ (Variables|Default|GetRotationAmount) (Math|Float|Clamp(Float) (.pitch (Transformation|GetWorldRotation (Variables|Default|GetSphere))) -9e+01 9e+01)) 0.0) false false))