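; BP_Cable is a cable actor whose spline mesh end point follows the mouse cursor once clicked.
; Clicking its capsule sets a Dragging flag, and Tick then moves the spline mesh end to the Visibility trace impact point under player 0's cursor.
; The release event is empty and nothing clears the flag, so the end keeps following after the button is released.
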(event OnClicked(Capsule)
  (params (TouchedComponent :type Primitive%20Component%20Object%20Reference) (ButtonPressed :type Key%20Structure :default "None"))
  (Variables|Default|SetDragging true))

(event OnReleased(Capsule)
  (params (TouchedComponent :type Primitive%20Component%20Object%20Reference) (ButtonReleased :type Key%20Structure :default "None")))

(event EventBeginPlay
  (Variables|Default|SetPlayerContREF (Game|GetPlayerController 0)))

(event Collision|EventActorBeginOverlap
  (params (OtherActor :type Actor%20Object%20Reference)))

(event EventTick
  (params (DeltaSeconds :type Float%20%28single-precision%29))
  (if (Variables|Default|GetDragging)
    (SplineMesh|SetEndPosition (Variables|Default|GetSplineMesh) (.impactpoint (.HitResult (Game|Player|GetHitResultUnderCursorbyChannel (Variables|Default|GetPlayerContREF) "TraceTypeQuery1" true))) true)))

(fn ConstructionScript)